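; BP_SplineAudio is an actor that makes a sound source follow the player along a spline.
; Each tick it finds the point on the Spline closest to the first player character's capsule and moves the Audio component there in world space.
; The update is skipped while the character's movement component reports falling, so the sound holds its last position during that time.
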(event EventTick
  (params (DeltaSeconds :type Float%20%28single-precision%29))
  (if (not (AI|Components|NavMovement|IsFalling (Variables|/Script/Engine.Character|GetCharacterMovement (Game|GetPlayerCharacter 0))))
    (Transformation|SetWorldLocation (Variables|Default|GetAudio) (Spline|FindLocationClosesttoWorldLocation (Variables|Default|GetSpline) (Transformation|GetWorldLocation (Variables|/Script/Engine.Character|GetCapsuleComponent (Game|GetPlayerCharacter 0))) "World") false false)))

(fn ConstructionScript)