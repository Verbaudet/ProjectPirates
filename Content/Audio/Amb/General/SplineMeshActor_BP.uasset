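; Ambient audio spline actor that keeps its Sea component alongside the player, apparently to emulate sea sound along a path.
; The construction script builds a spline mesh component for each spline segment.
; From BeginPlay, a self-repeating moveaudio event moves Sea every 0.05 seconds to the spline point closest to the cached FirstPersonCharacter, raised slightly in Z.
; A separate MoveAudio function graph is empty.
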(event Custom|moveaudio
  (bind _spline (Variables|Default|GetSpline))
  (bind _char_ref (Variables|Default|GetChar%20REF))
  (bind _returnvalue (Transformation|GetActorLocation _char_ref))
  (bind _returnvalue_2 (Spline|FindLocationClosesttoWorldLocation _spline _returnvalue "World"))
  (Transformation|SetWorldLocation (Variables|Default|GetSea) (Math|Vector|MakeVector (.x _returnvalue_2) (.y _returnvalue_2) (+ (.z _returnvalue_2) 5e+01)) false false)
  (Utilities|FlowControl|Delay 0.05)
  (CallFunction|Moveaudio))

(event EventBeginPlay
  (bind _asfirst_person_character (Utilities|Casting|CastToFirstPersonCharacter (Game|GetPlayerCharacter 0)))
  (Variables|Default|SetChar%20REF _asfirst_person_character)
  (CallFunction|Moveaudio))

(fn ConstructionScript
  (bind _spline (Variables|Default|GetSpline))
  (for _index (range 0 (- (Spline|GetNumberOfSplinePoints _spline) 2))
    (bind _returnvalue (AddComponent|AddSplineMeshComponent false))
    (Transformation|AttachComponentToComponent (Variables|SplineMeshActor|GetSplineMeshComponent) "None" "KeepRelative" "KeepRelative" "KeepRelative" true)
    (SplineMesh|SetStartandEnd _returnvalue (.Location (Spline|GetLocationandTangentatSplinePoint _spline _index "Local")) (.Tangent (Spline|GetLocationandTangentatSplinePoint _spline _index "Local")) (.Location (Spline|GetLocationandTangentatSplinePoint _spline (+ _index 1) "Local")) (.Tangent (Spline|GetLocationandTangentatSplinePoint _spline (+ _index 1) "Local")) true :!class /Script/Engine.SplineMeshComponent)))

(fn MoveAudio)